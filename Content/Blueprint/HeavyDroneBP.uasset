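; Heavy drone Blueprint that handles the drone's visual feedback for speed, lost state, command center changes and destruction.
; The construction script creates a dynamic material, and Tick drives its red channel from the speed ratio and turns the point light red when lost, otherwise green.
; A new command center triggers a spark effect that a timer later switches off, and destruction spawns an explosion emitter.
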(event `self.ReceiveTick`
  (params (DeltaSeconds :type "Float (single-precision)"))
  (bind _pointlight (`self.PointLight`))
  (`MaterialInstanceDynamic.SetVectorParameterValue` (`self.Dynamic Material H`) "Color" (make `LinearColor` (* (/ (`self.CurrentSpeed`) (`self.MaxSpeed`)) 256.0)))
  (if (`self.bIsLost`)
    (`LightComponent.SetLightColor` _pointlight (`KismetMathLibrary.LinearColor_Red`) true)
    (else
      (`LightComponent.SetLightColor` _pointlight (`KismetMathLibrary.LinearColor_Green`) true))))

(event `self.OnNewCommandCenter`
  (`ActorComponent.Activate` (`self.Spark`) false)
  (`KismetSystemLibrary.K2_SetTimerDelegate` (delegate `EmitSparks`) (`self.TimeSparkDelay`)))

(event `EmitSparks`
  (`ActorComponent.Deactivate` (`self.Spark`)))

(event `self.ReceiveDestroyed`
  (`GameplayStatics.SpawnEmitterAtLocation` "/Game/StarterContent/Particles/P_Explosion.P_Explosion" (`self.K2_GetActorLocation`)))

(fn `UserConstructionScript`
  (locals (`Dynamic Material` :type "MaterialInstanceDynamic Object Reference"))
  (bind _returnvalue (`PrimitiveComponent.CreateDynamicMaterialInstance` (`self.MeshComponent`) 0 "/Game/StarterContent/Materials/M_Basic_Wall.M_Basic_Wall" "None"))
  (set `self.Dynamic Material H` _returnvalue))